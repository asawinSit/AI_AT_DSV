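; BP_Bullet is a projectile that reports its hit outcome to the tank that fired it, feeding that tank's Q-learning.
; On BeginPlay it binds a handler to its sphere's component hit event.
; If the instigator is a BP_EnemyTank, it sets the Q-learning component's HitResult by whether the third-person character was struck, then calls Learn.
; The bullet destroys itself on any hit.
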(event Custom|CustomEvent
  (params (HitComponent :type Primitive%20Component%20Object%20Reference) (OtherActor :type Actor%20Object%20Reference) (OtherComp :type Primitive%20Component%20Object%20Reference) (NormalImpulse :type Vector) (Hit :type Hit%20Result%20Structure%20%28by%20ref%29))
  (bind _asbp_enemy_tank (Utilities|Casting|CastToBP_EnemyTank (Game|GetInstigator))
    (:then
      (Utilities|Casting|CastToBP_ThirdPersonCharacter OtherActor
        (:then
          (Variables|/Game/Blueprints/AI/BP_QLearningComponent.BP_QLearningComponent_C|SetHitResult (Variables|/Game/Blueprints/AI/BP_EnemyTank.BP_EnemyTank_C|GetBP_QLearningComponent _asbp_enemy_tank) true))
        (:CastFailed
          (Variables|/Game/Blueprints/AI/BP_QLearningComponent.BP_QLearningComponent_C|SetHitResult (Variables|/Game/Blueprints/AI/BP_EnemyTank.BP_EnemyTank_C|GetBP_QLearningComponent _asbp_enemy_tank) false)))
      (Default|Learn _asbp_enemy_tank)
      (Actor|DestroyActor))
    (:CastFailed
      (Actor|DestroyActor))))

(event EventBeginPlay
  (Collision|BindEventtoOnComponentHit (Variables|Default|GetSphere) (delegate Custom|CustomEvent)))

(event Collision|EventActorBeginOverlap
  (params (OtherActor :type Actor%20Object%20Reference)))

(event EventTick
  (params (DeltaSeconds :type Float%20%28single-precision%29)))

(fn ConstructionScript)