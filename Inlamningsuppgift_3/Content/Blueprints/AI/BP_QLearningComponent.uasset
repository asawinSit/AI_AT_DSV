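; AI component that implements tabular Q-learning, storing a value for each state-action pair so its user can choose actions.
; GetAction adds unseen states to the Q-table and greedily picks the highest-valued action; GetRandomAction separately picks one of five.
; UpdateQ nudges the stored value toward the reward by the learning rate, with no discounted next-state term.
; New states and value changes are broadcast through event dispatchers.
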(event EventBeginPlay)

(event EventTick
  (params (DeltaSeconds :type Float%20%28single-precision%29)))

(fn UpdateQ
  (params (State :type Enum_State%20Enum :default "NewEnumerator1") (Action :type Enum_Action%20Enum :default "NewEnumerator0") (Reward :type Float%20%28double-precision%29) (NewParam :type Float%20%28double-precision%29))
  (bind (_array_element _array_index) (Utilities|Array|ForEachLoopwithBreak (Variables|Default|GetQ-table) :!label _label)
    (:LoopBody
      (LocalVariables|SetActionsIndex _array_index)
      (if (Utilities|Enum|Equal(Enum) State (.state _array_element))
        (goto _label Break)))
    (:Completed
      (bind (_array_element_2 _array_index_2) (Utilities|Array|ForEachLoopwithBreak (.actions (Utilities|Array|Get(acopy) (Variables|Default|GetQ-table) (LocalVariables|GetActionsIndex))) :!label _label_2)
        (:LoopBody
          (LocalVariables|SetActionIndex _array_index_2)
          (if (Utilities|Enum|Equal(Enum) Action (.Action (Utilities|Struct|BreakActionValue _array_element_2)))
            (goto _label_2 Break)))
        (:Completed
          (bind _output_get (LocalVariables|SetNewQ (+ (* (Variables|Default|GetLearning%20rate) (- Reward (.qvalue (Utilities|Array|Get(acopy) (.actions (Utilities|Array|Get(acopy) (Variables|Default|GetQ-table) (LocalVariables|GetActionsIndex))) (LocalVariables|GetActionIndex))))) (.qvalue (Utilities|Array|Get(acopy) (.actions (Utilities|Array|Get(acopy) (Variables|Default|GetQ-table) (LocalVariables|GetActionsIndex))) (LocalVariables|GetActionIndex))))))
          (Utilities|Array|SetArrayElem (.actions (Utilities|Array|Get(acopy) (Variables|Default|GetQ-table) (LocalVariables|GetActionsIndex))) (LocalVariables|GetActionIndex) (Utilities|Struct|MakeActionValue (.action (Utilities|Array|Get(acopy) (.actions (Utilities|Array|Get(acopy) (Variables|Default|GetQ-table) (LocalVariables|GetActionsIndex))) (LocalVariables|GetActionIndex))) _output_get))
          (Default|CallQValueUpdated State (Utilities|Struct|MakeActionValue (.action (Utilities|Array|Get(acopy) (.actions (Utilities|Array|Get(acopy) (Variables|Default|GetQ-table) (LocalVariables|GetActionsIndex))) (LocalVariables|GetActionIndex))) _output_get))
          (return))))))

(fn GetQValue
  (params (State :type State%20Structure) (Action :type Action%20Value%20Structure))
  (if (Utilities|Array|ContainsItem (Variables|Default|GetQ-table) State)
    (if (Utilities|Array|ContainsItem (.Actions (Utilities|Struct|BreakState State)) Action)
      (return (.QValue (Utilities|Struct|BreakActionValue Action)))
      (else
        (return 0.0)))
    (else
      (return 0.0))))

(fn GetRandomAction
  (return (Utilities|Select :Index (Math|Random|RandomIntegerinRange 0 4) :Option%200 "NewEnumerator0" :Option%201 "NewEnumerator1" :Option%202 "NewEnumerator2" :Option%203 "NewEnumerator3" :Option%204 "NewEnumerator4")))

(fn GetAction
  (params (State :type Enum_State%20Enum :default "NewEnumerator1"))
  (bind _newlocalvar_0 (LocalVariables|GetNewLocalVar_0))
  (Utilities|FlowControl|Sequence
    (:then_0
      (bind _contains (CallFunction|QLearningContiansState State))
      (if (not _contains)
        (Utilities|Array|Add (Variables|Default|GetQ-table) (Utilities|Struct|MakeState State _newlocalvar_0))
        (Default|CallNewQLearningStateAdded (Utilities|Struct|MakeState State _newlocalvar_0))))
    (:then_1
      (bind (_array_element _array_index) (Utilities|Array|ForEachLoopwithBreak (Variables|Default|GetQ-table) :!label _label)
        (:LoopBody
          (LocalVariables|SetStateIndex _array_index)
          (if (Utilities|Enum|Equal(Enum) (.state _array_element) State)
            (goto _label Break)))
        (:Completed
          (bind _array_element_2 (Utilities|Array|ForEachLoopwithBreak (.Actions (Utilities|Struct|BreakState (Utilities|Array|Get(acopy) (Variables|Default|GetQ-table) (LocalVariables|GetStateIndex)))))
            (:LoopBody
              (bind _value (CallFunction|GetQValue (Utilities|Array|Get(acopy) (Variables|Default|GetQ-table) (LocalVariables|GetStateIndex)) _array_element_2))
              (if (> _value (LocalVariables|GetCurrentMax))
                (LocalVariables|SetCurrentMax _value)
                (LocalVariables|SetBestAction _array_element_2)))
            (:Completed
              (Utilities|FlowControl|Sequence
                (:then_1
                  (return (.action (LocalVariables|GetBestAction))))))))))))

(fn QLearningContiansState
  (params (State :type Enum_State%20Enum :default "NewEnumerator1"))
  (for _array_element (Variables|Default|GetQ-table)
    (if (Utilities|Enum|Equal(Enum) (.state _array_element) State)
      (return true)))
  (return false))