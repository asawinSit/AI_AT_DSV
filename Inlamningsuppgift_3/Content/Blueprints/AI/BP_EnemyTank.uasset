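; Enemy tank AI that senses targets, fires a cannon and can update a Q-learning component from shot results.
; Perception writes a sighted actor or heard location to the Blackboard and clears the target when a stimulus is lost.
; A fire event plays audio, briefly delays, then spawns a bullet from the muzzle along the gun's rotation.
; Learn rewards hits and penalizes misses when updating the Q-value for the last state and action.
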(event OnTargetPerceptionUpdated(AIPerception)
  (params (Actor :type Actor%20Object%20Reference) (Stimulus :type AI%20Stimulus%20Structure))
  (bind (_age _expirationage _strength _stimuluslocation _receiverlocation _tag _bsuccessfullysensed) (Utilities|Struct|BreakAIStimulus Stimulus))
  (bind _returnvalue (AI|GetBlackboard 0))
  (if _bsuccessfullysensed
    (bind _returnvalue_2 (Class|AIPerceptionSystem|GetSenseClassforStimulus Stimulus))
    (if (== _returnvalue_2 "/Script/AIModule.AISense_Sight")
      (Development|PrintString "enemy seen")
      (AI|Components|Blackboard|SetValueasObject _returnvalue (Utilities|Name|MakeLiteralName "TargetActor") Actor)
      (else
        (bind _returnvalue_3 (Class|AIPerceptionSystem|GetSenseClassforStimulus Stimulus))
        (if (== _returnvalue_3 "/Script/AIModule.AISense_Hearing")
          (AI|Components|Blackboard|SetValueasVector _returnvalue (Utilities|Name|MakeLiteralName "LastHeardLocation") _stimuluslocation))))
    (else
      (AI|Components|Blackboard|ClearValue (AI|GetBlackboard 0) (Utilities|Name|MakeLiteralName "TargetActor")))))

(event Custom|Event_FireCannon
  (Audio|Components|Audio|Play (Variables|Default|GetTankShotAudio) 0.0)
  (Utilities|FlowControl|Delay 0.1)
  (CallFunction|Shoot))

(fn ConstructionScript)

(fn Shoot
  (bind _self self)
  (bind _returnvalue (Game|SpawnActorfromClass "/Game/ThirdPerson/Blueprints/BP_Bullet.BP_Bullet_C" (Math|Transform|MakeTransform (Transformation|GetWorldLocation (Variables|Default|GetMuzzlePoint)) (Transformation|GetWorldRotation (Variables|Default|GetSM_tank_gun_001)) "1.000000,1.000000,1.000000") "Undefined" "MultiplyWithRoot" _self _self))
  (Variables|Default|SetHitActor 0)
  (Variables|Default|SetCurrentShot _returnvalue))

(fn Learn
  (bind _bp_qlearningcomponent (Variables|Default|GetBP_QLearningComponent))
  (Utilities|FlowControl|Sequence
    (:then_0
      (if (Variables|/Game/Blueprints/AI/BP_QLearningComponent.BP_QLearningComponent_C|GetHitResult _bp_qlearningcomponent)
        (LocalVariables|SetNewLocalVar 1.0)
        (else
          (LocalVariables|SetNewLocalVar -0.1))))
    (:then_1
      (Default|UpdateQ _bp_qlearningcomponent (Variables|/Game/Blueprints/AI/BP_QLearningComponent.BP_QLearningComponent_C|GetLastState _bp_qlearningcomponent) (Variables|/Game/Blueprints/AI/BP_QLearningComponent.BP_QLearningComponent_C|GetLastAction _bp_qlearningcomponent) (LocalVariables|GetNewLocalVar) 0.0))))